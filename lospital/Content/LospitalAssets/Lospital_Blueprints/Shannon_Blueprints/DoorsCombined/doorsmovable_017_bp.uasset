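; Double door Blueprint that swings two door meshes open and closed as the HazmatCharacter passes through its trigger volumes.
; Entering the Enter volume plays the Doors timeline, which scales AngleA and AngleB into relative yaw on DoorAExit and DoorBExit.
; Leaving Enter reverses the timeline.
; Overlapping Exit also reverses it, but only the first time, as its DoOnce is never reset.
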(event OnComponentBeginOverlap(enter)
  (params (OverlappedComponent :type Primitive%20Component%20Object%20Reference) (OtherActor :type Actor%20Object%20Reference) (OtherComp :type Primitive%20Component%20Object%20Reference) (OtherBodyIndex :type Integer) (bFromSweep :type Boolean) (SweepResult :type Hit%20Result%20Structure%20%28by%20ref%29))
  (Utilities|Casting|CastToHazmatCharacter OtherActor)
  (bind _newtrack_0 (Timeline|doors Play)
    (:Update
      (Transformation|SetRelativeRotation (Variables|Default|GetDoorAExit) (Math|Rotator|MakeRotator 0.0 0.0 (* _newtrack_0 (Variables|Default|GetAngle_A))) false false)
      (Transformation|SetRelativeRotation (Variables|Default|GetDoorBExit) (Math|Rotator|MakeRotator 0.0 0.0 (* _newtrack_0 (Variables|Default|GetAngle_B))) false false))))

(event OnComponentEndOverlap(enter)
  (params (OverlappedComponent :type Primitive%20Component%20Object%20Reference) (OtherActor :type Actor%20Object%20Reference) (OtherComp :type Primitive%20Component%20Object%20Reference) (OtherBodyIndex :type Integer))
  (Utilities|Casting|CastToHazmatCharacter OtherActor)
  (bind _newtrack_0 (Timeline|doors Reverse)
    (:Update
      (Transformation|SetRelativeRotation (Variables|Default|GetDoorAExit) (Math|Rotator|MakeRotator 0.0 0.0 (* _newtrack_0 (Variables|Default|GetAngle_A))) false false)
      (Transformation|SetRelativeRotation (Variables|Default|GetDoorBExit) (Math|Rotator|MakeRotator 0.0 0.0 (* _newtrack_0 (Variables|Default|GetAngle_B))) false false))))

(event OnComponentBeginOverlap(exit)
  (params (OverlappedComponent :type Primitive%20Component%20Object%20Reference) (OtherActor :type Actor%20Object%20Reference) (OtherComp :type Primitive%20Component%20Object%20Reference) (OtherBodyIndex :type Integer) (bFromSweep :type Boolean) (SweepResult :type Hit%20Result%20Structure%20%28by%20ref%29))
  (Utilities|Casting|CastToHazmatCharacter OtherActor)
  (Utilities|FlowControl|DoOnce false
    (:Completed
      (bind _newtrack_0 (Timeline|doors Reverse)
        (:Update
          (Transformation|SetRelativeRotation (Variables|Default|GetDoorAExit) (Math|Rotator|MakeRotator 0.0 0.0 (* _newtrack_0 (Variables|Default|GetAngle_A))) false false)
          (Transformation|SetRelativeRotation (Variables|Default|GetDoorBExit) (Math|Rotator|MakeRotator 0.0 0.0 (* _newtrack_0 (Variables|Default|GetAngle_B))) false false))))))

(event OnComponentEndOverlap(exit)
  (params (OverlappedComponent :type Primitive%20Component%20Object%20Reference) (OtherActor :type Actor%20Object%20Reference) (OtherComp :type Primitive%20Component%20Object%20Reference) (OtherBodyIndex :type Integer)))

(event EventBeginPlay)

(event Collision|EventActorBeginOverlap
  (params (OtherActor :type Actor%20Object%20Reference)))

(event EventTick
  (params (DeltaSeconds :type Float%20%28single-precision%29)))

(fn ConstructionScript)