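; Trigger volume that switches on the hall ceiling lights when the HazmatCharacter overlaps its box.
; The overlap runs two sequence branches that each fetch every Rectlight_ceiling_bp actor in the level and make its root component visible, without propagating to children.
; The branches differ only in delay, half a second versus one second, so the second pass repeats the first on the same lights.
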(event OnComponentBeginOverlap(Box)
  (params (OverlappedComponent :type Primitive%20Component%20Object%20Reference) (OtherActor :type Actor%20Object%20Reference) (OtherComp :type Primitive%20Component%20Object%20Reference) (OtherBodyIndex :type Integer) (bFromSweep :type Boolean) (SweepResult :type Hit%20Result%20Structure%20%28by%20ref%29))
  (Utilities|Casting|CastToHazmatCharacter OtherActor)
  (Utilities|FlowControl|Sequence
    (:then_0
      (bind _outactors (Actor|GetAllActorsOfClass "/Game/LospitalAssets/Lospital_Blueprints/Shannon_Blueprints/DoorsCombined/rectlight_ceiling_bp.rectlight_ceiling_bp_C"))
      (Utilities|FlowControl|Delay 0.5)
      (for _array_element _outactors
        (Rendering|SetVisibility (Variables|/Script/Engine.Actor|GetRootComponent _array_element) true false)))
    (:then_1
      (bind _outactors_2 (Actor|GetAllActorsOfClass "/Game/LospitalAssets/Lospital_Blueprints/Shannon_Blueprints/DoorsCombined/rectlight_ceiling_bp.rectlight_ceiling_bp_C"))
      (Utilities|FlowControl|Delay 1.0)
      (for _array_element_2 _outactors_2
        (Rendering|SetVisibility (Variables|/Script/Engine.Actor|GetRootComponent _array_element_2) true false)))))

(event EventBeginPlay)

(event Collision|EventActorBeginOverlap
  (params (OtherActor :type Actor%20Object%20Reference)))

(event EventTick
  (params (DeltaSeconds :type Float%20%28single-precision%29)))

(fn ConstructionScript)