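; BP_PuzzleLight is a puzzle light actor that lets the player toggle its point light with the Z key while inside a trigger box.
; Trigger overlap enables or disables input for player controller 0 and toggles the prompt text's visibility, without checking which actor overlapped.
; The construction script applies the prompt's location, rotation and initial visibility from variables, allowing setup per instance.
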(event OnComponentBeginOverlap(TriggerBox)
  (params (OverlappedComponent :type Primitive%20Component%20Object%20Reference) (OtherActor :type Actor%20Object%20Reference) (OtherComp :type Primitive%20Component%20Object%20Reference) (OtherBodyIndex :type Integer) (bFromSweep :type Boolean) (SweepResult :type Hit%20Result%20Structure%20%28by%20ref%29))
  ;[0.6021 0.2952 1] Enables key input and shows text on trigger overlap
  (Input|EnableInput (Game|GetPlayerController 0))
  (Rendering|ToggleVisibility (Variables|Default|GetPlayerInputText) false))

(event OnComponentEndOverlap(TriggerBox)
  (params (OverlappedComponent :type Primitive%20Component%20Object%20Reference) (OtherActor :type Actor%20Object%20Reference) (OtherComp :type Primitive%20Component%20Object%20Reference) (OtherBodyIndex :type Integer))
  ;[0.6021 0.2952 1] Enables key input and shows text on trigger overlap
  (Input|DisableInput (Game|GetPlayerController 0))
  (Rendering|ToggleVisibility (Variables|Default|GetPlayerInputText) false))

(event Input|KeyboardEvents|Z
  (params (Key :type Key%20Structure :default "None"))
  ;[1 0.263 0.4613] Toggles light while inside trigger box with "z"
  (:Pressed
    (Rendering|ToggleVisibility (Variables|Default|GetPointLight) false)))

(fn ConstructionScript
  ;[0.1444 1 0.8069] Sets up text location and visibility parameters for instances
  (Transformation|SetRelativeLocationAndRotation (Variables|Default|GetPlayerInputText) (Variables|Default|GetTextLocation) (Variables|Default|GetTextRotation) false false)
  (Rendering|SetVisibility (Variables|Default|GetPlayerInputText) (Variables|Default|GetIsVisible?) false))